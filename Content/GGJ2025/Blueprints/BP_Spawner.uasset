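; Spawner that builds a vertically stacked level at runtime from random level clusters, loaded as streaming level instances.
; BeginPlay loads the first cluster, picking a random DT_LevelClusters row that matches CurrentDifficulty.
; Each SpawnNextLevel call requests unload of the last level, shifts the last/current/next references, and loads a new cluster at Z offset TotalHeight, accumulated from cluster heights.
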(event Custom|Spawn%20Next%20Level
  (Utilities|FlowControl|Sequence
    (:then_0
      (Utilities|IsValid (Variables|Livelli|GetLast%20Level)
        (:Is%20Valid
          (Class|LevelStreaming|SetIsRequestingUnloadandRemoval (Variables|Livelli|GetLast%20Level) true))
        (:Is%20Not%20Valid
          _))
      (Variables|Livelli|SetLast%20Level (Variables|Livelli|GetCurrent%20Level))
      (Variables|Livelli|SetCurrent%20Level (Variables|Levels|GetNext%20Level)))
    (:then_1
      (Variables|LevelDatas|SetCurrent%20Level%20Datas (Variables|LevelDatas|GetNext%20Level%20Datas))
      (Variables|Livelli|SetCurrent%20Level (Variables|Levels|GetNext%20Level))
      (bind _outitem (CallFunction|ChoseRandomLevelbyDifficulty (Variables|Default|GetCurrent%20Difficulty)))
      (bind _returnvalue (Utilities|GetDataTableRow "/Game/GGJ2025/DT_LevelClusters.DT_LevelClusters" _outitem)
        (:then
          (Variables|LevelDatas|SetNext%20Level%20Datas _returnvalue)
          (bind _output_get (Variables|Default|SetTotal%20Height (+ (Variables|Default|GetTotal%20Height) (.height (Variables|LevelDatas|GetCurrent%20Level%20Datas)))))
          (bind (_boutsuccess _returnvalue_2) (Class|LevelStreamingDynamic|LoadLevelInstance (.levelassetname (Variables|LevelDatas|GetNext%20Level%20Datas)) (Math|Vector|MakeVector 0.0 0.0 _output_get) "0, 0, 0" "" 0 false))
          (if _boutsuccess
            (Variables|Levels|SetNext%20Level _returnvalue_2)))))))

(event EventBeginPlay
  (Variables|LevelDatas|SetCurrent%20Level%20Datas (Variables|LevelDatas|GetNext%20Level%20Datas))
  (Variables|Livelli|SetCurrent%20Level (Variables|Levels|GetNext%20Level))
  (bind _outitem (CallFunction|ChoseRandomLevelbyDifficulty (Variables|Default|GetCurrent%20Difficulty)))
  (bind _returnvalue (Utilities|GetDataTableRow "/Game/GGJ2025/DT_LevelClusters.DT_LevelClusters" _outitem)
    (:then
      (Variables|LevelDatas|SetNext%20Level%20Datas _returnvalue)
      (bind _output_get (Variables|Default|SetTotal%20Height (+ (Variables|Default|GetTotal%20Height) (.height (Variables|LevelDatas|GetCurrent%20Level%20Datas)))))
      (bind (_boutsuccess _returnvalue_2) (Class|LevelStreamingDynamic|LoadLevelInstance (.levelassetname (Variables|LevelDatas|GetNext%20Level%20Datas)) (Math|Vector|MakeVector 0.0 0.0 _output_get) "0, 0, 0" "" 0 false))
      (if _boutsuccess
        (Variables|Levels|SetNext%20Level _returnvalue_2)))))

(fn ConstructionScript)

(fn ChoseRandomLevelbyDifficulty
  (params (Difficulty :type Integer))
  (bind _outrownames (DataTable|GetDataTableRowNames "/Game/GGJ2025/DT_LevelClusters.DT_LevelClusters"))
  (for _array_element _outrownames
    (bind _returnvalue (Utilities|GetDataTableRow "/Game/GGJ2025/DT_LevelClusters.DT_LevelClusters" _array_element)
      (:then
        (if (== (.difficulty _returnvalue) Difficulty)
          (Utilities|Array|Add (LocalVariables|GetAcceptable%20Levels) _array_element)))))
  (return (.OutItem (Utilities|Array|Random (LocalVariables|GetAcceptable%20Levels)))))