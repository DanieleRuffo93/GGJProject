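; BP_SpawnGM is a game-mode Blueprint that owns the level spawning and ranking managers.
; On BeginPlay it spawns BP_Spawner and BP_RankingMNG far below the world origin and keeps references to both.
; Interface-style events forward next-level requests to the spawner and collectible score additions to the ranking manager.
; A custom SAD event triggers the same next-level spawn.
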(event Custom|SAD
  (Default|SpawnNextLevel (Variables|MNGs|GetSpawn%20MNG)))

(event EventBeginPlay
  (CallFunction|ConstructManagers))

(event EventIAddCollectiblesScore
  (params (Score%20to%20Add :type Integer))
  ;[0.15 0.15 0.15 0.5] Ranking
  (Default|AddCollectibleScore (Variables|MNGs|GetRanking%20MNG) Score%20to%20Add))

(event EventISpawnNextLevel
  (Default|SpawnNextLevel (Variables|MNGs|GetSpawn%20MNG)))

(fn ConstructionScript)

(fn ConstructManagers
  (bind _returnvalue (Game|SpawnActorfromClass "/Game/GGJ2025/GameplayFramework/Blueprints/BP_Spawner.BP_Spawner_C" (Math|Transform|MakeTransform "0.000000,0.000000,-100000.000000" "0, 0, 0" "1.000000,1.000000,1.000000") "AlwaysSpawn" "MultiplyWithRoot" self 0))
  (Variables|MNGs|SetSpawn%20MNG _returnvalue)
  (bind _returnvalue_2 (Game|SpawnActorfromClass "/Game/GGJ2025/UI/BP_RankingMNG.BP_RankingMNG_C" (Math|Transform|MakeTransform "0.000000,0.000000,-100000.000000" "0, 0, 0" "1.000000,1.000000,1.000000") "AlwaysSpawn" "MultiplyWithRoot" self 0))
  (Variables|MNGs|SetRanking%20MNG _returnvalue_2))