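; Game Instance for the GGJ 2025 game that holds audio settings and the music timeline position, exposed through interface calls.
; It spawns the audio manager actor with the stored settings, then forwards FMOD music and SFX parameters and volume changes to it.
; The music position is saved from the manager's speaker.
; Setting that position does nothing here, and the music parameter getter always returns zero.
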(event EventISetAudioSettings
  (params (Audio%20Settings :type S%20Audio%20Settings%20Structure))
  (Variables|Default|SetAudio%20Settings Audio%20Settings))

(event EventISetVolumeSettings
  (params (AudioSettings :type S%20Audio%20Settings%20Structure))
  (bind _output_get (Variables|Default|SetAudio%20Settings AudioSettings))
  (Default|ChangeVolumesSettings (Variables|Default|GetAudio%20MNG) _output_get))

(event EventISetFMODSFXParameter
  (params (Name :type Name :default "None") (Value :type Float%20%28double-precision%29))
  (Default|SetFMODSFXParamater (Variables|Default|GetAudio%20MNG) Name Value))

(event EventISetFMODMusicParameter
  (params (Name :type Name :default "None") (Value :type Float%20%28double-precision%29))
  (Default|SetFMODMusicParameter (Variables|Default|GetAudio%20MNG) Name Value))

(event EventISpawnAudioManager
  (bind _returnvalue (Game|SpawnActorfromClass "/Game/GGJ2025/GameplayFramework/Blueprints/BP_AudioMng.BP_AudioMng_C" (Math|Transform|MakeTransform "0.000000,0.000000,-100.000000" "0, 0, 0" "1.000000,1.000000,1.000000") "AlwaysSpawn" "MultiplyWithRoot" 0 (Variables|Default|GetAudio%20Settings) 0))
  (Variables|Default|SetAudio%20MNG _returnvalue))

(event EventISetMusicTimelinePos
  (params (_Timeline%20Pos :type Integer) (Set%20Current? :type Boolean))
  (if Set%20Current?
    _))

(event EventISaveMusicTimelinePos
  (bind _returnvalue (Class|FMODAudioComponent|GetTimelinePosition (Variables|/Game/GGJ2025/GameplayFramework/Blueprints/BP_AudioMng.BP_AudioMng_C|GetMusicSpeaker (Variables|Default|GetAudio%20MNG))))
  (Variables|Default|SetMusic%20Timeline%20Position _returnvalue))

(fn IGetAudioSettings
  (return (Variables|Default|GetAudio%20Settings)))

(fn IGetAudioManager
  (return (Variables|Default|GetAudio%20MNG)))

(fn IGetFMODMusicParameter
  (params (Name :type Name :default "None"))
  (return 0.0))

(fn IGetMusicTimelinePos
  (return (Variables|Default|GetMusic%20Timeline%20Position)))

(fn IGetVolumeSettings
  (return (Variables|Default|GetAudio%20Settings)))