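; BP_Eraser is a rising hazard that climbs along Z and erases whatever its capsule overlaps.
; Tick moves it with a sweep at Speed, which a Play/Stop event toggles between stopped and moving.
; It also drives the FMOD "Danger" music parameter, which grows as the player's height lead shrinks within SafeDistance.
; Any overlap sends an Erase interface message to the other actor and sets the "Death" music parameter.
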(event OnComponentBeginOverlap(Capsule)
  (params (OverlappedComponent :type Primitive%20Component%20Object%20Reference) (OtherActor :type Actor%20Object%20Reference) (OtherComp :type Primitive%20Component%20Object%20Reference) (OtherBodyIndex :type Integer) (bFromSweep :type Boolean) (SweepResult :type Hit%20Result%20Structure%20%28by%20ref%29))
  (Class|IErasable|IErase(Message) OtherActor)
  (Class|IAudioController|ISetFMODMusicParameter(Message) (Game|GetGameInstance) "Death" 1.0))

(event Custom|Play/Stop
  (Utilities|FlowControl|FlipFlop
    (:A
      (Variables|Default|SetSpeed 0.0))
    (:B
      (Variables|Default|SetSpeed 4e+02))))

(event EventTick
  (params (DeltaSeconds :type Float%20%28single-precision%29))
  (bind _returnvalue (Transformation|GetActorLocation))
  (Transformation|SetActorLocation (Math|Vector|MakeVector (.x _returnvalue) (.y _returnvalue) (+ (.z _returnvalue) (* DeltaSeconds (Variables|Default|GetSpeed)))) true false)
  (Class|IAudioController|ISetFMODMusicParameter(Message) (Game|GetGameInstance) "Danger" (Math|Float|Lerp 1e+01 1.0 (/ (Math|Float|Clamp(Float) (- (.z (Transformation|GetActorLocation (Game|Player|GetPlayerPawn 0))) (.z (Transformation|GetActorLocation))) 0.0 (Variables|Default|GetSafe%20Distance)) (Variables|Default|GetSafe%20Distance)))))

(fn ConstructionScript)