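; BP_AudioMng is an audio manager that plays the game's FMOD music and exposes volume and parameter controls.
; On BeginPlay it reads audio settings from the GameInstance via an interface, then starts the OST at main times music volume.
; Timelines drive volume changes, though music updates skip the lerp and SFX updates target MusicSpeaker.
; Separate events forward named parameters to MusicSpeaker and SFXSpeaker.
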(event Custom|Change%20Music%20Volume
  (params (volume :type Float%20%28single-precision%29))
  (bind _returnvalue (Math|Float|Clamp(Float) volume))
  ;[0.15 0.15 0.15 0.5] Volumes
  (bind _alpha (Timeline|TL_ChangeMusicVolume PlayFromStart)
    (:Update
      (Class|FMODAudioComponent|SetVolume (Variables|Default|GetMusicSpeaker) _returnvalue))
    (:Finished
      (Variables|Default|SetMusicVolume (Math|Float|Lerp (Variables|Default|GetMusicVolume) _returnvalue _alpha)))))

(event Custom|Change%20SFX%20Volume
  (params (Value :type Float%20%28double-precision%29))
  ;[0.15 0.15 0.15 0.5] Volumes
  (bind _alpha (Timeline|TL_ChangeSFXVolume PlayFromStart)
    (:Update
      (Class|FMODAudioComponent|SetVolume (Variables|Default|GetMusicSpeaker) (Math|Float|Lerp (Variables|Default|GetSFXVolume) (Math|Float|Clamp(Float) Value) _alpha)))
    (:Finished
      (Variables|Default|SetSFXVolume (Math|Float|Lerp (Variables|Default|GetSFXVolume) (Math|Float|Clamp(Float) Value) _alpha)))))

(event Custom|sadas
  (bind _finalvalue (Class|FMODAudioComponent|GetParameterValue (Variables|Default|GetMusicSpeaker) "LVL"))
  (Development|PrintString (Utilities|String|ToString(Float) _finalvalue)))

(event Custom|Set%20FMOD%20Music%20Parameter
  (params (Name :type Name) (Value :type Float%20%28single-precision%29))
  (Class|FMODAudioComponent|SetParameter (Variables|Default|GetMusicSpeaker) Name Value))

(event Custom|Set%20FMOD%20SFX%20Paramater
  (params (Name :type Name) (Value :type Float%20%28single-precision%29))
  (Class|FMODAudioComponent|SetParameter (Variables|Default|GetSFXSpeaker) Name Value))

(event EventBeginPlay
  (bind _musicspeaker (Variables|Default|GetMusicSpeaker))
  (Utilities|FlowControl|Sequence
    (:then_0
      (bind _audio_settings (Class|ISaver|IGetAudioSettings(Message) (Game|GetGameInstance)))
      (Variables|Default|SetOST%20Settings _audio_settings))
    (:then_1
      (Class|FMODAudioComponent|SetEvent _musicspeaker "/Game/FMOD/Events/OST.OST")
      (Class|FMODAudioComponent|Play (Variables|Default|GetMusicSpeaker))
      (Class|FMODAudioComponent|SetVolume _musicspeaker (* (.mainvolume (Variables|Default|GetOST%20Settings)) (.musicvolume (Variables|Default|GetOST%20Settings)))))))

(fn ConstructionScript)