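; BP_Spawner is an actor that streams stacked level instances with rising difficulty and spawns enemies around the player's orbit area.
; SpawnNextLevel unloads the older level and loads a random or mandatory one from DT_DifficultyStats at accumulated height.
; Completed-level counts raise difficulty and the FMOD music parameter.
; A looping timer spawns random enemies on a ring at player-relative height; the initial level setup is unconnected.
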(event Custom|Spawn%20Next%20Level
  (Math|Integer|IncrementInt (Variables|DifficultyStats|GetCompleted%20Levels)
    (:%20%20
      (CallFunction|CheckDifficulty)
      (Utilities|FlowControl|Sequence
        (:then_0
          (Utilities|IsValid (Variables|Livelli|GetLast%20Level)
            (:Is%20Valid
              (Class|LevelStreaming|SetIsRequestingUnloadandRemoval (Variables|Livelli|GetLast%20Level) true))
            (:Is%20Not%20Valid
              _))
          (Variables|Livelli|SetLast%20Level (Variables|Livelli|GetCurrent%20Level)))
        (:then_1
          (CallFunction|LevelSpawn))))))

(event Custom|Level%20Spawn
  (Variables|Default|SetCurrent%20Lv%20Datas (Variables|LevelDatas|GetNext%20Level%20Datas))
  (Variables|Livelli|SetCurrent%20Level (Variables|Levels|GetNext%20Level))
  (CallFunction|LevelChoiceMethod)
  (bind _output_get (Variables|Default|SetTotal%20Height (+ (Variables|Default|GetTotal%20Height) (.Height (Utilities|Struct|BreakLevelSpawnData (Variables|Default|GetCurrent%20Lv%20Datas))))))
  (bind (_boutsuccess _returnvalue) (Class|LevelStreamingDynamic|LoadLevelInstance (.levelassetname (Variables|LevelDatas|GetNext%20Level%20Datas)) (Math|Vector|MakeVector 0.0 0.0 _output_get) "0, 0, 0" "" 0 true))
  (if _boutsuccess
    (Variables|Levels|SetNext%20Level _returnvalue)))

(event Custom|DEBUG%20Set%20LVL%20to%201
  (Class|IAudioController|ISetFMODMusicParameter(Message) (Game|GetGameInstance) "LVL" (Math|Conversions|ToFloat(Integer) (+ (Variables|DifficultyStats|GetCurrent%20Difficulty) 1))))

(event Custom|Spawn%20Enemy
  (bind (_center _sqrradius) (Class|SuperellipseOrbitComponent|GetCenterandSqrRadius (Variables|Default|GetOrbit)))
  (bind _output_get (Variables|Default|SetEnemy%20To%20Spawn (.OutItem (Utilities|Array|Random (Variables|Default|GetEnemy%20Classes)))))
  (bind _returnvalue (Game|SpawnActorfromClass _output_get (Math|Transform|MakeTransform (+ (Math|Vector|MakeVector (.x _center) (.y _center) (+ (.z (Transformation|GetActorLocation (Game|Player|GetPlayerPawn 0))) (Variables|Default|GetEnemy%20Spawn%20VOffset))) (* (* _sqrradius 0.495) (Math|Vector|Normalize (Math|Vector|MakeVector (Math|Random|RandomFloatinRange -1e+01 1e+01) (Math|Random|RandomFloatinRange -1e+01 1e+01) 0.0)))) "0, 0, 0" "1.000000,1.000000,1.000000") "AdjustIfPossibleButDontSpawnIfColliding" "MultiplyWithRoot" 0 0))
  (Utilities|Array|Add (Variables|Default|GetEnemies) _returnvalue))

(event Custom|Start%20Enemy%20Spawn
  (bind _returnvalue (Utilities|Time|SetTimerbyEvent (delegate Custom|Spawn%20Enemy) (Variables|Default|GetEnemy%20Spawn%20Time) true))
  (Variables|Default|SetEnemy%20Spawn%20Timer _returnvalue)
  (bind _orbit (Class|IOrbitOrigin|IGetOrbit(Message) (Game|GetGameMode)))
  (Variables|Default|SetOrbit _orbit))

(event EventBeginPlay)

(fn ConstructionScript)

(fn CheckDifficulty
  (if (and (>= (Variables|DifficultyStats|GetCompleted%20Levels) (Variables|DifficultyStats|GetCurrent%20Difficulty%20Level%20Num)) (> (Variables|DifficultyStats|GetMax%20Difficulty) (Variables|DifficultyStats|GetCurrent%20Difficulty)))
    (bind _result (Math|Integer|IncrementInt (Variables|DifficultyStats|GetCurrent%20Difficulty))
      (:%20%20
        (CallFunction|SetDifficulty _result)
        (Class|IAudioController|ISetFMODMusicParameter(Message) (Game|GetGameInstance) "LVL" (Math|Conversions|ToFloat(Integer) (+ (Variables|DifficultyStats|GetCurrent%20Difficulty) 1)))))))

(fn SetDifficulty
  (params (Difficulty :type Integer))
  (bind _output_get (Variables|DifficultyStats|SetCurrent%20Difficulty Difficulty))
  (bind _returnvalue (Utilities|GetDataTableRow "/Game/GGJ2025/GameplayFramework/Datas/DT_DifficultyStats.DT_DifficultyStats" (Utilities|String|StringToName (Utilities|String|ToString(Integer) _output_get)))
    (:then
      (bind _output_get_2 (Variables|DifficultyStats|SetCurrent%20Difficulty%20Level%20Num (Math|Random|RandomIntegerinRange (.min (.LevelsToOvercome (Utilities|Struct|BreakS_DifficultyStats _returnvalue))) (.max (.LevelsToOvercome (Utilities|Struct|BreakS_DifficultyStats _returnvalue))))))
      (Development|PrintString (Utilities|String|Append "You need " (Utilities|String|ToString(Integer) _output_get_2) " levels to go to next difficulty")))
    (:RowNotFound
      (Development|PrintString "Selected Difficulty is not implemented"))))

(fn LevelChoiceMethod
  (bind _returnvalue (Utilities|GetDataTableRow "/Game/GGJ2025/GameplayFramework/Datas/DT_DifficultyStats.DT_DifficultyStats" (Utilities|String|StringToName (Utilities|String|ToString(Integer) (Variables|DifficultyStats|GetCurrent%20Difficulty))))
    (:then
      (if (not (Utilities|Map|Contains (.mandatoryindex-level _returnvalue) (Variables|DifficultyStats|GetCompleted%20Levels)))
        (Variables|LevelDatas|SetNext%20Level%20Datas (.OutItem (Utilities|Array|Random (.levels _returnvalue))))
        (else
          (Variables|LevelDatas|SetNext%20Level%20Datas (.Value (Utilities|Map|Find (.mandatoryindex-level _returnvalue) (Variables|DifficultyStats|GetCompleted%20Levels))))))
      (return))))