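; BP_BaseEnemy is the base enemy character, providing a behavior tree, FMOD audio scaled by game-mode volume settings, and timed distance-based despawning.
; Capsule overlaps send the other actor a damage message with an outward impulse.
; Received hits are cooldown-gated, spawning a random onomatopoeia Niagara tile toward the camera with its matching sound.
; The enemy then becomes a physics body, is launched, and after a delay plays death audio and is destroyed.
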(event OnComponentBeginOverlap(Capsule)
  (params (OverlappedComponent :type Primitive%20Component%20Object%20Reference) (OtherActor :type Actor%20Object%20Reference) (OtherComp :type Primitive%20Component%20Object%20Reference) (OtherBodyIndex :type Integer) (bFromSweep :type Boolean) (SweepResult :type Hit%20Result%20Structure%20%28by%20ref%29))
  (bind _returnvalue (Transformation|GetActorLocation))
  (bind _returnvalue_2 (Transformation|GetActorLocation OtherActor))
  (bind _returnvalue_3 (- _returnvalue_2 _returnvalue))
  (bind _returnvalue_4 (Math|Vector|Normalize _returnvalue_3))
  ;[0.15 0.15 0.15 0.5] Take Damage
  (Class|IDamageable|ITakeDamage(Message) OtherActor (* (Math|Vector|MakeVector (.x _returnvalue_4) (.y _returnvalue_4) (.z _returnvalue_4)) (Variables|Default|GetImpulse%20Force))))

(event Custom|Damage:%20Mechanic
  (params (LaunchVelocity :type Vector))
  ;[0.15 0.15 0.15 0.5] Take Damage
  (Collision|SetCollisionEnabled (Variables|Default|GetCapsule) "NoCollision")
  (Physics|SetSimulatePhysics (Variables|Default|GetCapsuleComponent) true)
  (Physics|AddImpulse (Variables|Default|GetCapsuleComponent) LaunchVelocity "None" true)
  (Utilities|FlowControl|Delay (Variables|Danno|GetTime%20to%20Die))
  (Class|FMODAudioComponent|SetEvent (Variables|Default|GetFMODAudio) "/Game/FMOD/Events/SFX/Enemies_Death.Enemies_Death")
  (Class|FMODAudioComponent|Play (Variables|Default|GetFMODAudio))
  (Actor|DestroyActor))

(event Custom|Damage::%20Graphic
  (bind _returnvalue (Transformation|GetActorLocation))
  ;[0.15 0.15 0.15 0.5] Take Damage
  (CallFunction|ChoseOnomat)
  (bind _returnvalue_2 (Niagara|SpawnSystematLocation "/Game/GGJ2025/VFX/OnomaTOPEEEEE/NS_OnomatopeicDamage.NS_OnomatopeicDamage" (+ (* (Math|Vector|Normalize (- (Camera|GetCameraLocation (Game|GetPlayerCameraManager 0)) _returnvalue)) (Variables|Default|GetOnomat%20VFX%20Distance)) _returnvalue) "0, 0, 0" "1.000000,1.000000,1.000000" true true "AutoRelease"))
  (Class|NiagaraComponent|SetVariableVec2 _returnvalue_2 "Tile" (.Tile (Utilities|Struct|BreakS_OnomatTiles (Variables|Danno|GetDamage%20Tile)))))

(event Custom|Chose%20Onomat
  ;[0.15 0.15 0.15 0.5] Take Damage
  (Variables|Danno|SetDamage%20Tile (.OutItem (Utilities|Array|Random (Variables|Danno|GetDamage%20Tiles)))))

(event Custom|Damage:%20Sound
  ;[0.15 0.15 0.15 0.5] Take Damage
  (Class|FMODBlueprintStatics|PlayEvent2D (.sound (Variables|Danno|GetDamage%20Tile))))

(event Custom|Check%20For%20Despawn
  (if (<= (Variables|Default|GetDespawnDistance) (Math|Vector|VectorLengthSquared (- (Transformation|GetActorLocation) (Transformation|GetActorLocation (Game|Player|GetPlayerPawn 0)))))
    (Actor|DestroyActor)))

(event Custom|Start%20Despawn%20Check
  (Utilities|Time|SetTimerbyEvent (delegate Custom|Check%20For%20Despawn) (Variables|Default|GetDespawn%20Check%20Period) true))

(event EventIPlaySoundfromAgent
  (params (Sound :type FMOD%20Event%20Object%20Reference) (Play%20Standard%20Sound? :type Boolean))
  ;[0.15 0.15 0.15 0.5] Take Damage
  (if Play%20Standard%20Sound?
    (bind _audio_settings (Class|ISaver|IGetAudioSettings(Message) (Game|GetGameMode)))
    (Class|FMODAudioComponent|SetVolume (Variables|Default|GetFMODAudio) (* (.mainvolume _audio_settings) (* (.sfxvolume _audio_settings) 0.25)))
    (Class|FMODAudioComponent|Play (Variables|Default|GetFMODAudio))))

(event EventBeginPlay
  (Utilities|Time|SetTimerbyEvent (delegate Custom|Start%20Despawn%20Check) 2e+01)
  (Class|FMODAudioComponent|SetEvent (Variables|Default|GetFMODAudio) "/Game/FMOD/Events/SFX/Enemies.Enemies")
  (bind _audiosettings (Class|IAudioController|IGetVolumeSettings(Message) (Game|GetGameMode)))
  (Class|FMODAudioComponent|SetVolume (Variables|Default|GetFMODAudio) (* (* (.mainvolume _audiosettings) (.sfxvolume _audiosettings)) 0.85))
  (Class|FMODAudioComponent|Play (Variables|Default|GetFMODAudio)))

(event EventITakeDamage
  (params (Hit%20Direction :type Vector :default "0, 0, 0"))
  ;[0.15 0.15 0.15 0.5] Take Damage
  (if (> (- (Utilities|Time|GetTimeSeconds) (Variables|Damage|GetLast%20Hit%20Time)) (Variables|Danno|GetTime%20To%20Hit%20Again))
    (Variables|Damage|SetLast%20Hit%20Time (Utilities|Time|GetTimeSeconds))
    (CallFunction|Damage::Graphic)
    (CallFunction|Damage:Sound)
    (CallFunction|Damage:Mechanic Hit%20Direction)))

(fn ConstructionScript)

(fn IGetBehaviorTree
  (return (Variables|Default|GetBT)))