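; Enemy Blueprint that reacts to hits with randomized onomatopoeia effects and sound, with the damage mechanic left as an empty stub.
; Capsule overlap, ITakeDamage and PlaytakeDamage share one hit path, throttled by a time cooldown.
; Each hit picks a random DamageTile, spawns a pooled Niagara effect offset toward the camera using that tile, then plays its paired 2D sound.
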(event OnComponentBeginOverlap(CapsuleComponent)
  (params (OverlappedComponent :type Primitive%20Component%20Object%20Reference) (OtherActor :type Actor%20Object%20Reference) (OtherComp :type Primitive%20Component%20Object%20Reference) (OtherBodyIndex :type Integer) (bFromSweep :type Boolean) (SweepResult :type Hit%20Result%20Structure%20%28by%20ref%29))
  ;[0.15 0.15 0.15 0.5] Take Damage
  (if (> (- (Utilities|Time|GetTimeSeconds) (Variables|Default|GetLast%20Hit%20Time)) (Variables|Default|GetTime%20To%20Hit%20Again))
    (Variables|Default|SetLast%20Hit%20Time (Utilities|Time|GetTimeSeconds))
    (CallFunction|Damage:Mechanic)
    (CallFunction|Damage::Graphic)
    (CallFunction|Damage:Sound)))

(event Custom|Damage:%20Mechanic
  ;[0.15 0.15 0.15 0.5] Take Damage
)

(event Custom|Damage::%20Graphic
  (bind _returnvalue (Transformation|GetActorLocation))
  ;[0.15 0.15 0.15 0.5] Take Damage
  (CallFunction|ChoseOnomat)
  (bind _returnvalue_2 (Niagara|SpawnSystematLocation "/Game/GGJ2025/VFX/OnomaTOPEEEEE/NS_OnomatopeicDamage.NS_OnomatopeicDamage" (+ (* (Math|Vector|Normalize (- (Camera|GetCameraLocation (Game|GetPlayerCameraManager 0)) _returnvalue)) (Variables|Default|GetOnomat%20VFX%20Distance)) _returnvalue) "0, 0, 0" "1.000000,1.000000,1.000000" true true "AutoRelease"))
  (Class|NiagaraComponent|SetVariableVec2 _returnvalue_2 "Tile" (.Tile (Utilities|Struct|BreakS_OnomatTiles (Variables|Default|GetDamage%20Tile)))))

(event Custom|Chose%20Onomat
  (Variables|Default|SetDamage%20Tile (.OutItem (Utilities|Array|Random (Variables|Default|GetDamage%20Tiles)))))

(event Custom|Damage:%20Sound
  ;[0.15 0.15 0.15 0.5] Take Damage
  (Class|FMODBlueprintStatics|PlayEvent2D (.sound (Variables|Default|GetDamage%20Tile))))

(event Custom|Play%20take%20Damage
  ;[0.15 0.15 0.15 0.5] Take Damage
  (if (> (- (Utilities|Time|GetTimeSeconds) (Variables|Default|GetLast%20Hit%20Time)) (Variables|Default|GetTime%20To%20Hit%20Again))
    (Variables|Default|SetLast%20Hit%20Time (Utilities|Time|GetTimeSeconds))
    (CallFunction|Damage:Mechanic)
    (CallFunction|Damage::Graphic)
    (CallFunction|Damage:Sound)))

(event EventITakeDamage
  ;[0.15 0.15 0.15 0.5] Take Damage
  (if (> (- (Utilities|Time|GetTimeSeconds) (Variables|Default|GetLast%20Hit%20Time)) (Variables|Default|GetTime%20To%20Hit%20Again))
    (Variables|Default|SetLast%20Hit%20Time (Utilities|Time|GetTimeSeconds))
    (CallFunction|Damage:Mechanic)
    (CallFunction|Damage::Graphic)
    (CallFunction|Damage:Sound)))

(fn ConstructionScript)