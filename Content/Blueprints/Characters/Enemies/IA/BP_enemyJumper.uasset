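; Nav link blueprint that makes AI characters jump across when they reach its smart link.
; On SmartLinkReached it stores the agent as LastPathWalker, solves a high-arc toss velocity toward a point slightly above the destination, and launches the character with it.
; The projectile solver traces the full path, accepts the closest solution and draws debug.
; Custom-arc and path-prediction alternatives remain in the graph but never run.
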(event EventSmartLinkReached
  (params (Agent :type Actor%20Object%20Reference) (Destination :type Vector%20%28by%20ref%29 :default "0, 0, 0"))
  (bind _aspersonaggio (Utilities|Casting|CastToCharacter Agent))
  (Variables|Default|SetLast%20Path%20Walker _aspersonaggio)
  (bind _tossvelocity (Class|GameplayStatics|BlueprintSuggestProjectileVelocity (Transformation|GetActorLocation (Variables|Default|GetLast%20Path%20Walker)) (+ Destination "0.000000,0.000000,100.000000") 6e+02 0.0 "TraceFullPath" 1.8e+02 true true true))
  (Character|LaunchCharacter (Variables|Default|GetLast%20Path%20Walker) _tossvelocity true true))

(fn ConstructionScript)