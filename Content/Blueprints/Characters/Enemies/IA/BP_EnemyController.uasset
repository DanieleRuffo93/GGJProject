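; Enemy AI controller that runs the behavior tree supplied by its possessed pawn and feeds it patrol positions.
; After a short delay on possess, it starts the tree and seeds the Blackboard with the player pawn, the game mode's Orbit object and an initial patrol location.
; An interface function cycles through the pawn's patrol actors with a wrapping index, returning the next location or a zero vector if none exist.
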(event EventPossess
  (params (PossessedPawn :type Pawn%20Object%20Reference))
  (Variables|Default|SetPossessed%20Pawn PossessedPawn)
  (Utilities|FlowControl|Delay 2.5)
  (bind _bt (Class|IAIAgent|IGetBehaviorTree(Message) PossessedPawn))
  (AI|RunBehaviorTree _bt)
  (AI|Components|Blackboard|SetValueasObject (AI|GetBlackboard 0) (Utilities|Name|MakeLiteralName "Player") (Game|Player|GetPlayerPawn 0))
  (bind _orbit (Class|IOrbitOrigin|IGetOrbit(Message) (Game|GetGameMode)))
  (AI|Components|Blackboard|SetValueasObject (AI|GetBlackboard 0) (Utilities|Name|MakeLiteralName "Orbit") _orbit)
  (bind _pat_positions (Class|IAIAgent|IGetPatrolPositions(Message) (Variables|Default|GetPossessed%20Pawn)))
  (if (Utilities|Array|IsNotEmpty _pat_positions)
    (AI|Components|Blackboard|SetValueasVector (AI|GetBlackboard 0) (Utilities|Name|MakeLiteralName "PatrolPositions") (Transformation|GetActorLocation (Utilities|Array|Get(acopy) _pat_positions (Variables|Default|GetPatrol%20Index))))))

(fn ConstructionScript)

(fn IGetNextPatrolPosition
  (bind _pat_positions (Class|IAIAgent|IGetPatrolPositions(Message) (Variables|Default|GetPossessed%20Pawn)))
  (LocalVariables|SetPP%20Arr _pat_positions)
  (bind _result (Math|Integer|IncrementInt (Variables|Default|GetPatrol%20Index))
    (:%20%20
      (if (Utilities|Array|IsNotEmpty (LocalVariables|GetPP%20Arr))
        (return (Transformation|GetActorLocation (Utilities|Array|Get(acopy) (LocalVariables|GetPP%20Arr) (Math|Integer|%(Integer) _result (Utilities|Array|Length _pat_positions)))))
        (else
          (return "0, 0, 0"))))))