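; Enemy Blueprint that reacts to damage, either from a collider overlap or through a TakeDamage interface event, with comic-style onomatopoeia effects.
; Both triggers share one chain that runs separate mechanic, graphic and sound events, of which only the graphic is implemented.
; The graphic event spawns an auto-released pooled Niagara system at the actor's location and passes a randomly chosen tile as a Vec2 parameter to vary the displayed word.
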(event OnComponentBeginOverlap(Collider)
  (params (OverlappedComponent :type Primitive%20Component%20Object%20Reference) (OtherActor :type Actor%20Object%20Reference) (OtherComp :type Primitive%20Component%20Object%20Reference) (OtherBodyIndex :type Integer) (bFromSweep :type Boolean) (SweepResult :type Hit%20Result%20Structure%20%28by%20ref%29))
  ;[0.15 0.15 0.15 0.5] Take Damage
  (CallFunction|Damage:Mechanic (stale EventITakeDamage Damage%20Amount))
  (CallFunction|Damage::Graphic)
  (CallFunction|Damage:Sound))

(event Custom|Damage:%20Mechanic
  (params (Damage%20Amount :type Float%20%28double-precision%29))
  ;[0.15 0.15 0.15 0.5] Take Damage
)

(event Custom|Damage::%20Graphic
  ;[0.15 0.15 0.15 0.5] Take Damage
  (CallFunction|ChoseOnomat)
  (bind _returnvalue (Niagara|SpawnSystematLocation "/Game/GGJ2025/VFX/OnomaTOPEEEEE/NS_OnomatopeicDamage.NS_OnomatopeicDamage" (Transformation|GetActorLocation) "0, 0, 0" "1.000000,1.000000,1.000000" true true "AutoRelease"))
  (Class|NiagaraComponent|SetVariableVec2 _returnvalue "Tile" (.Tile (Utilities|Struct|BreakS_OnomatTiles (Variables|Default|GetDamage%20Tile)))))

(event Custom|Chose%20Onomat
  (Variables|Default|SetDamage%20Tile (.OutItem (Utilities|Array|Random (Variables|Default|GetDamage%20Tiles)))))

(event Custom|Damage:%20Sound
  ;[0.15 0.15 0.15 0.5] Take Damage
)

(event EventITakeDamage
  (params (Damage%20Amount :type Float%20%28double-precision%29))
  ;[0.15 0.15 0.15 0.5] Take Damage
  (CallFunction|Damage:Mechanic Damage%20Amount)
  (CallFunction|Damage::Graphic)
  (CallFunction|Damage:Sound))

(fn ConstructionScript)