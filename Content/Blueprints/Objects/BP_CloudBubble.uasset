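; BP_CloudBubble is an object Blueprint that launches any Character overlapping it, using its LaunchVelocity variable.
; Both the actor-level overlap event and the Collider component's begin-overlap event cast the other actor to Character and call LaunchCharacter with identical logic.
; Both XY and Z overrides are off, so the launch adds to the character's existing velocity.
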(event OnComponentBeginOverlap(Collider)
  (params (OverlappedComponent :type Primitive%20Component%20Object%20Reference) (OtherActor :type Actor%20Object%20Reference) (OtherComp :type Primitive%20Component%20Object%20Reference) (OtherBodyIndex :type Integer) (bFromSweep :type Boolean) (SweepResult :type Hit%20Result%20Structure%20%28by%20ref%29))
  (bind _ascharacter (Utilities|Casting|CastToCharacter OtherActor))
  (Character|LaunchCharacter _ascharacter (Variables|Default|GetLaunch%20Velocity) false false))

(event EventBeginPlay
  (|CallParentFunction) ; This node is disabled and will not be called.\nDrag off pins to build functionality.
)

(event Collision|EventActorBeginOverlap
  (params (OtherActor :type Actor%20Object%20Reference))
  (bind _ascharacter (Utilities|Casting|CastToCharacter OtherActor))
  (Character|LaunchCharacter _ascharacter (Variables|Default|GetLaunch%20Velocity) false false))

(fn ConstructionScript
  (|CallParentFunction))