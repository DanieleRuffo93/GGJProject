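; BP_PlugBubble is a bubble object that knocks back what touches it and shows random phrases.
; Actor overlap launches Characters along their reversed forward vector, with horizontal speed scaling only Y and an offset subtracted from Z.
; Collider overlap sends the other actor a take-damage interface message carrying an upward impulse directed away from the player pawn.
; ChangePhrase sets both text renders from a random pick of Texts.
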(event OnComponentBeginOverlap(Collider)
  (params (OverlappedComponent :type Primitive%20Component%20Object%20Reference) (OtherActor :type Actor%20Object%20Reference) (OtherComp :type Primitive%20Component%20Object%20Reference) (OtherBodyIndex :type Integer) (bFromSweep :type Boolean) (SweepResult :type Hit%20Result%20Structure%20%28by%20ref%29))
  (bind _returnvalue (Transformation|GetActorLocation OtherActor))
  (bind _returnvalue_2 (Game|Player|GetPlayerPawn 0))
  (bind _returnvalue_3 (Transformation|GetActorLocation _returnvalue_2))
  (bind _returnvalue_4 (- _returnvalue _returnvalue_3))
  (bind _returnvalue_5 (Math|Vector|Normalize _returnvalue_4))
  (Class|IDamageable|ITakeDamage(Message) OtherActor (* (Math|Vector|MakeVector (.x _returnvalue_5) (.y _returnvalue_5) 1.0) (Variables|Default|GetImpulse%20Strenght))))

(event Custom|Change%20Phrase
  (Rendering|Components|TextRender|SetText (Variables|Default|GetTextRender) (.OutItem (Utilities|Array|Random (Variables|Default|GetTexts)))))

(event EventBeginPlay
  (|CallParentFunction) ; This node is disabled and will not be called.\nDrag off pins to build functionality.
)

(event Collision|EventActorBeginOverlap
  (params (OtherActor :type Actor%20Object%20Reference))
  (bind _aspersonaggio (Utilities|Casting|CastToCharacter OtherActor))
  (Character|LaunchCharacter _aspersonaggio (Math|Vector|MakeVector (.x (Math|Vector|NegateVector (Transformation|GetActorForwardVector _aspersonaggio))) (* (Variables|Default|GetLaunch%20%20Horizontal%20Speed) (.y (Math|Vector|NegateVector (Transformation|GetActorForwardVector _aspersonaggio)))) (- (.z (Math|Vector|NegateVector (Transformation|GetActorForwardVector _aspersonaggio))) (Variables|Default|GetLaunch%20Vertical%20Speed%20Offset))) false false))

(fn ConstructionScript
  (|CallParentFunction))