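; Bubble component that places a reusable bubble platform in front of the player.
; SpawnBubble shows the existing Bubble's platform, enables its collision and plays a 2D activation sound.
; It then moves the Bubble ahead of the player, adding an air offset when falling, and calls DespawnBubble.
; When grounded on a floor of the GameTraceChannel1 object type, it skips the move and despawn call.
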(event Custom|SpawnBubble
  (bind _returnvalue (Game|GetPlayerCharacter 0))
  (bind _returnvalue_2 (Game|GetPlayerCharacter 0))
  (bind _distance_from_player_ (Variables|Gameplay|GetDistance%20from%20player%20))
  (bind _bubble (Variables|References|GetBubble))
  (bind _returnvalue_3 (Transformation|GetActorLocation _returnvalue_2))
  (bind _returnvalue_4 (Transformation|GetActorForwardVector _returnvalue_2))
  (bind _bubbleplatform (Variables|/Game/Blueprints/Objects/BP_Bubble.BP_Bubble_C|GetBubblePlatform _bubble))
  (bind _charactermovement (Variables|/Script/Engine.Character|GetCharacterMovement _returnvalue))
  (bind _returnvalue_5 (* _returnvalue_4 _distance_from_player_))
  (bind _returnvalue_6 (+ _returnvalue_3 _returnvalue_5))
  (Rendering|SetVisibility _bubbleplatform true false)
  (Collision|SetCollisionEnabled _bubbleplatform "QueryAndPhysics")
  (Class|FMODBlueprintStatics|PlayEvent2D "/Game/FMOD/Events/SFX/Platform_On.Platform_On")
  (if (AI|Components|NavMovement|IsFalling _charactermovement)
    (Transformation|SetActorLocation (Variables|References|GetBubble) (+ _returnvalue_6 (Variables|Gameplay|GetSpawnOffsetOnAir)) false false)
    (Default|DespawnBubble (Variables|References|GetBubble) :!label _label)
    (elif (not (Utilities|Enum|Equal(Enum) (Collision|GetCollisionObjectType (.HitComponent (Collision|BreakHitResult (.HitResult (Utilities|Struct|BreakFindFloorResult (Variables|/Script/Engine.CharacterMovementComponent|GetCurrentFloor _charactermovement)))))) "ECC_GameTraceChannel1"))
      (Transformation|SetActorLocation (Variables|References|GetBubble) _returnvalue_6 false false)
      (goto _label))))