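; Component that places the solid bubble in front of the player character.
; Its SpawnSolidBubble event moves the existing SolidBubble actor to a set distance along player 0's forward vector rather than creating a new one.
; When the character is falling, it adds an air spawn offset to that position.
; The move is neither swept nor a physics teleport.
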(event Custom|SpawnSolidBubble
  (bind _returnvalue (Game|GetPlayerCharacter 0))
  (bind _distance_from_player_ (Variables|Gameplay|GetDistance%20from%20player%20))
  (bind _returnvalue_2 (Transformation|GetActorLocation _returnvalue))
  (bind _returnvalue_3 (Transformation|GetActorForwardVector _returnvalue))
  (bind _returnvalue_4 (* _returnvalue_3 _distance_from_player_))
  (bind _returnvalue_5 (+ _returnvalue_2 _returnvalue_4))
  (if (AI|Components|NavMovement|IsFalling (Variables|/Script/Engine.Character|GetCharacterMovement (Game|GetPlayerCharacter 0)))
    (Transformation|SetActorLocation (Variables|References|GetSolidBubble) (+ _returnvalue_5 (Variables|Gameplay|GetSpawnOffsetOnAir)) false false)
    (else
      (Transformation|SetActorLocation (Variables|References|GetSolidBubble) _returnvalue_5 false false))))